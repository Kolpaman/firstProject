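; BP_Door is an interactable door that toggles between open and closed.
; On interact, it waits briefly, then flips IsDoorOpen and plays or reverses the DoorOpen timeline.
; The timeline's OpenDoor track drives the door's relative yaw to animate the swing.
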(event `/Game/FirstPerson/Blueprints/BI_Interaction.Event Interact`
  (`KismetSystemLibrary.Delay` 0.3)
  (if (not (`self.IsDoorOpen?`))
    (set `self.IsDoorOpen?` true)
    (bind (_direction _open_door) (`Timeline|Door Open` :!label _label)
      (:`Update`
        (`SceneComponent.K2_SetRelativeRotation` (`self.Door`) (`KismetMathLibrary.MakeRotator` 0.0 0.0 _open_door) false false)))
    (else
      (set `self.IsDoorOpen?` false)
      (goto _label :!via `Reverse`))))

(fn `UserConstructionScript`
  (`parent.UserConstructionScript`))