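; BP_LightSwitch is an interactable wall switch that toggles a linked spotlight on and off.
; Each interact event runs a FlipFlop that plays a flick sound at the switch and sets the light's spotlight intensity on or to zero.
; The RotateTime timeline plays forward or in reverse to lerp the switch mesh's pitch, animating the flip.
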(event `/Game/FirstPerson/Blueprints/BI_Interaction.Event Interact`
  (bind _returnvalue (`SceneComponent.K2_GetComponentLocation` (`self.Switch`)))
  (bind _spotlightcomponent (`SpotLight.SpotLightComponent` (`self.light`)))
  (`/Engine/EditorBlueprintResources/StandardMacros.FlipFlop`
    (:`A`
      (`GameplayStatics.PlaySoundAtLocation` "/Game/Interface_And_Item_Sounds/WAV/Flick_Switch_03.Flick_Switch_03" _returnvalue (struct) 1.0 1.0 0.0 null null null null)
      (`LightComponent.SetIntensity` _spotlightcomponent 1000.0)
      (bind (_direction _lightswitchalpha) (`Timeline|rotate time` :!label _label)
        (:`Update`
          (`SceneComponent.K2_SetRelativeRotation` (`self.Switch`) (`KismetMathLibrary.MakeRotator` 0.0 (`KismetMathLibrary.Lerp` 0.0 45.0 _lightswitchalpha) 90.0) false false))))
    (:`B`
      (`GameplayStatics.PlaySoundAtLocation` "/Game/Interface_And_Item_Sounds/WAV/Flick_Switch_03.Flick_Switch_03" _returnvalue (struct) 1.0 1.0 0.0 null null null null)
      (`LightComponent.SetIntensity` _spotlightcomponent 0.0)
      (goto _label :!via `Reverse`))))

(fn `UserConstructionScript`
  (`parent.UserConstructionScript`))